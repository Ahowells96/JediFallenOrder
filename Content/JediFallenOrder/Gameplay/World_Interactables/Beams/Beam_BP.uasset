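; Walkable balance beam actor that puts a ThirdPersonCharacter onto a spline path when it enters from either end.
; The construction script builds spline meshes along the spline and moves the end trigger and arrow to the last point.
; Start and end trigger overlaps toggle the character's OnBeam state, setting the path, entry direction and a starting distance just inside that end.
; Movement along the beam is not handled here.
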(event `self.TriggerStart.OnComponentBeginOverlap`
  (params (OverlappedComponent :type "PrimitiveComponent Object Reference") (OtherActor :type "Actor Object Reference") (OtherComp :type "PrimitiveComponent Object Reference") (OtherBodyIndex :type Integer) (bFromSweep :type Boolean) (SweepResult :type "HitResult Structure (by ref)"))
  (bind _asthird_person_character (cast `/Game/ThirdPersonBP/Blueprints/ThirdPersonCharacter` OtherActor))
  (set `/Game/ThirdPersonBP/Blueprints/ThirdPersonCharacter.EnteredBackwards` false _asthird_person_character)
  (if (`/Game/ThirdPersonBP/Blueprints/ThirdPersonCharacter.OnBeam?` _asthird_person_character)
    (set `/Game/ThirdPersonBP/Blueprints/ThirdPersonCharacter.OnBeam?` false _asthird_person_character)
    (else
      (set `/Game/ThirdPersonBP/Blueprints/ThirdPersonCharacter.SplinePath` self _asthird_person_character)
      (set `/Game/ThirdPersonBP/Blueprints/ThirdPersonCharacter.DistanceAlongSpline` 60.0 _asthird_person_character)
      (set `/Game/ThirdPersonBP/Blueprints/ThirdPersonCharacter.OnBeam?` true _asthird_person_character))))

(event `self.TriggerEnd.OnComponentBeginOverlap`
  (params (OverlappedComponent :type "PrimitiveComponent Object Reference") (OtherActor :type "Actor Object Reference") (OtherComp :type "PrimitiveComponent Object Reference") (OtherBodyIndex :type Integer) (bFromSweep :type Boolean) (SweepResult :type "HitResult Structure (by ref)"))
  (bind _asthird_person_character (cast `/Game/ThirdPersonBP/Blueprints/ThirdPersonCharacter` OtherActor))
  (set `/Game/ThirdPersonBP/Blueprints/ThirdPersonCharacter.EnteredBackwards` true _asthird_person_character)
  (if (`/Game/ThirdPersonBP/Blueprints/ThirdPersonCharacter.OnBeam?` _asthird_person_character)
    (set `/Game/ThirdPersonBP/Blueprints/ThirdPersonCharacter.OnBeam?` false _asthird_person_character)
    (else
      (bind _output_get (set `/Game/ThirdPersonBP/Blueprints/ThirdPersonCharacter.SplinePath` self _asthird_person_character))
      (set `/Game/ThirdPersonBP/Blueprints/ThirdPersonCharacter.DistanceAlongSpline` (- (`SplineComponent.GetSplineLength` (`/Game/JediFallenOrder/Gameplay/World_Interactables/Beams/Beam_BP.Spline` _output_get)) 60.0) _asthird_person_character)
      (set `/Game/ThirdPersonBP/Blueprints/ThirdPersonCharacter.OnBeam?` true _asthird_person_character))))

(fn `UserConstructionScript`
  (bind _returnvalue_location (`KismetMathLibrary.BreakTransform` (`KismetMathLibrary.MakeTransform` (0.0 0.0 50.0))))
  (bind _spline (`self.Spline`))
  (bind _spline_2 (`self.Spline`))
  (bind (_returnvalue_location_2 _returnvalue_rotation) (`KismetMathLibrary.BreakTransform` (`SplineComponent.GetTransformAtSplinePoint` _spline_2 (`SplineComponent.GetNumberOfSplinePoints` _spline_2) "World" false)))
  ;[1 1 1] Spline Creation
  (for _index (range (+ (- (`SplineComponent.GetNumberOfSplinePoints` _spline) 2) 1))
    (bind _returnvalue (`AddComponent|NODE_AddSplineMeshComponent-0` :`RelativeTransform` (`KismetMathLibrary.MakeTransform` (0.0 0.0 -25.0))))
    (`SceneComponent.K2_AttachToComponent` _returnvalue (`self.DefaultSceneRoot`) "None" "KeepRelative" "KeepRelative" "KeepRelative" true)
    (bind (_location _tangent) (`SplineComponent.GetLocationAndTangentAtSplinePoint` _spline _index "Local"))
    (bind (_location_2 _tangent_2) (`SplineComponent.GetLocationAndTangentAtSplinePoint` _spline (+ _index 1) "Local"))
    (`SplineMeshComponent.SetStartAndEnd` _returnvalue _location _tangent _location_2 _tangent_2 true)
    (`SceneComponent.K2_SetWorldTransform` (`self.TriggerEnd`) (`KismetMathLibrary.MakeTransform` (+ _returnvalue_location_2 _returnvalue_location) _returnvalue_rotation) false false)
    (`SceneComponent.K2_SetWorldTransform` (`self.Arrow`) (`KismetMathLibrary.MakeTransform` _returnvalue_location_2 _returnvalue_rotation) false false)))